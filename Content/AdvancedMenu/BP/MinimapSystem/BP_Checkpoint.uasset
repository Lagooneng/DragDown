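; BP_Checkpoint is a world checkpoint that shows an icon and its distance to the player, plus a matching minimap icon.
; On BeginPlay it sets up its widget component, creates a minimap icon widget and attaches a CalcHelper component to the player's root.
; Each Tick it moves CalcHelper to the checkpoint, using its relative location as the player-relative minimap position.
; Tick also updates the distance text in whole meters.
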(event `self.ReceiveBeginPlay`
  (bind _aswdg_checkpoint (cast `/Game/AdvancedMenu/BP/MinimapSystem/WDG_Checkpoint` (`WidgetComponent.GetWidget` (`self.Widget checkpoint`))))
  (bind _output_get (set `self.Wdg Checkpoint` _aswdg_checkpoint))
  (`/Game/AdvancedMenu/BP/MinimapSystem/WDG_Checkpoint.UpdateIcon` _output_get (`self.icon`) (40.0 40.0))
  (`KismetSystemLibrary.Delay` 0.2)
  (bind _returnvalue (`|CreateWidget` "/Game/AdvancedMenu/BP/MinimapSystem/WDG_MinimapIcon.WDG_MinimapIcon_C"))
  (bind _output_get_2 (set `self.minimap icon` _returnvalue))
  (`/Game/AdvancedMenu/BP/MinimapSystem/WDG_MinimapIcon.ChangeIcon` _output_get_2 (`self.icon`))
  (`/Game/AdvancedMenu/BP/MinimapSystem/WDG_MinimapIcon.Change Size` _output_get_2 (`self.icon size`))
  (`UserWidget.AddToViewport` _output_get_2 0)
  (`SceneComponent.K2_AttachToComponent` (`self.calc_helper`) (`Actor.RootComponent` (`GameplayStatics.GetPlayerCharacter` 0)) "None" "KeepWorld" "KeepWorld" "KeepWorld" true)
  (`self.UpdateIconPosition`))

(event `self.ReceiveTick`
  (params (DeltaSeconds :type "Float (single-precision)"))
  (`self.UpdateIconPosition`)
  (`/Game/AdvancedMenu/BP/MinimapSystem/WDG_Checkpoint.Set Text` (`self.Wdg Checkpoint`) (`KismetTextLibrary.Conv_IntToText` (`KismetMathLibrary.FTrunc` (/ (`KismetMathLibrary.Vector_Distance` (`self.K2_GetActorLocation` (`GameplayStatics.GetPlayerCharacter` 0)) (`self.K2_GetActorLocation`)) 100.0)))))

(fn `UpdateIconPosition`
  (`SceneComponent.K2_SetWorldLocation` (`self.calc_helper`) (`self.K2_GetActorLocation`) false false)
  (bind _minimap_icon (`self.minimap icon`)
    (:`then`
      (`/Game/AdvancedMenu/BP/MinimapSystem/WDG_MinimapIcon.UpdateIconLocation` _minimap_icon (`KismetMathLibrary.Conv_VectorToVector2D` (`SceneComponent.RelativeLocation` (`self.calc_helper`))) 0.0))
    (:`else`)))

(fn `UserConstructionScript`)