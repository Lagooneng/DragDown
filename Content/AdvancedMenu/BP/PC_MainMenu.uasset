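; PC_MainMenu is a player controller for the advanced menu that relays pause input and captures keys for control rebinding.
; The Pause Game action sends the HUD a PauseGameMessage carrying the inverse of the current paused state.
; RegisterKeyChange stores a control widget, which receives the next pressed key through OnAnyKey and is then cleared, making each capture one-shot.
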(event `InputAction|Pause Game` :paused true
  (params (Key :type "Key Structure"))
  ;[1 1 1] PauseGame
  (:`Pressed`
    (message `/Game/AdvancedMenu/BP/Interfaces/BPI_HUD.PauseGame` (`self.GetHUD`) (not (`GameplayStatics.IsGamePaused`)))))

(event `/Game/AdvancedMenu/BP/Interfaces/BPI_PlayerController.RegisterKeyChange`
  (params (`wdg control` :type "/Game/AdvancedMenu/BP/UI/WDG_controls_04 Object Reference"))
  ;[1 1 1] Controls
  (set `self.Wdg Control` `wdg control`))

(event `Key|AnyKey` :consume false :paused true
  (params (Key :type "Key Structure"))
  (bind _wdg_control (`self.Wdg Control`))
  ;[1 1 1] Controls
  (:`Pressed`
    (`/Engine/EditorBlueprintResources/StandardMacros.IsValid` _wdg_control
      (:`Is Valid`
        (`/Game/AdvancedMenu/BP/UI/WDG_controls_04.OnAnyKey` _wdg_control Key)
        (set `self.Wdg Control` null)))))

(fn `UserConstructionScript`)