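; BP_CaveCross is a configurable cave crossing piece for the Western desert town environment, with no active runtime logic.
; Its construction script sets meshes from two enum choices: ceiling decoration with optional beams, and wall decoration with optional supports.
; Option 2 in either choice always includes the beams or supports.
; It also toggles two direction visualizers and shows or hides three dust particle components, passing them a shared density parameter.
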(fn `UserConstructionScript`
  (bind _particles2 (`self.Particles2`))
  (bind _particles3 (`self.Particles3`))
  (bind _particles1 (`self.Particles1`))
  (bind _visualize_direction (`self.Visualize Direction`))
  (`|ExecutionSequence`
    (:`then_0`
      (`|ExecutionSequence`
        (:`then_0`
          (`SceneComponent.SetVisibility` (`self.Direction1`) _visualize_direction false))
        (:`then_1`
          (`SceneComponent.SetVisibility` (`self.Direction2`) _visualize_direction false))))
    (:`then_1`
      (switch `/Game/WesternDesertTown/Blueprint/BlueprintExtra/ENUM_CeilingType` (`self.Ceiling Decoration`)
        (:`NewEnumerator1`
          (`StaticMeshComponent.SetStaticMesh` (`self.Beams`) "/Game/WesternDesertTown/Mesh/CaveModules/CaveSupport/SM_CrossBeams.SM_CrossBeams" :!label _label))
        (:`NewEnumerator2`
          (`|ExecutionSequence`
            (:`then_0`
              (goto _label))
            (:`then_1`
              (`StaticMeshComponent.SetStaticMesh` (`self.CeilingDecoration`) "/Game/WesternDesertTown/Mesh/CaveModules/CaveDecoration/SM_CrossCeiling01.SM_CrossCeiling01" :!label _label_2))))
        (:`NewEnumerator3`
          (goto _label_2))
        (:`NewEnumerator4`
          (`StaticMeshComponent.SetStaticMesh` (`self.CeilingDecoration`) "/Game/WesternDesertTown/Mesh/CaveModules/CaveDecoration/SM_CrossCeiling02.SM_CrossCeiling02")
          (`StaticMeshComponent.SetStaticMesh` (`self.Beams`) "/Game/WesternDesertTown/Mesh/CaveModules/CaveSupport/SM_CrossBeams.SM_CrossBeams"))))
    (:`then_2`
      (switch `/Game/WesternDesertTown/Blueprint/BlueprintExtra/ENUM_WallsType` (`self.Wall Decoration`)
        (:`NewEnumerator1`
          (`StaticMeshComponent.SetStaticMesh` (`self.Supports`) "/Game/WesternDesertTown/Mesh/CaveModules/CaveSupport/SM_CrossSupports.SM_CrossSupports" :!label _label_3))
        (:`NewEnumerator2`
          (`|ExecutionSequence`
            (:`then_0`
              (goto _label_3))
            (:`then_1`
              (`StaticMeshComponent.SetStaticMesh` (`self.WallsDecoration`) "/Game/WesternDesertTown/Mesh/CaveModules/CaveDecoration/SM_CrossWalls01.SM_CrossWalls01" :!label _label_4))))
        (:`NewEnumerator3`
          (goto _label_4))
        (:`NewEnumerator4`
          (`StaticMeshComponent.SetStaticMesh` (`self.WallsDecoration`) "/Game/WesternDesertTown/Mesh/CaveModules/CaveDecoration/SM_CrossWalls02.SM_CrossWalls02")
          (`StaticMeshComponent.SetStaticMesh` (`self.Supports`) "/Game/WesternDesertTown/Mesh/CaveModules/CaveSupport/SM_CrossSupports.SM_CrossSupports"))))
    (:`then_3`
      (`|ExecutionSequence`
        (:`then_0`
          (`SceneComponent.SetVisibility` _particles1 (`self.Enable Dust Particles`) false)
          (`FXSystemComponent.SetFloatParameter` _particles1 "Density" (`self.Dust Particles Density`)))
        (:`then_1`
          (`SceneComponent.SetVisibility` _particles2 (`self.Enable Dust Particles`) false)
          (`FXSystemComponent.SetFloatParameter` _particles2 "Density" (`self.Dust Particles Density`)))
        (:`then_2`
          (`SceneComponent.SetVisibility` _particles3 (`self.Enable Dust Particles`) false)
          (`FXSystemComponent.SetFloatParameter` _particles3 "Density" (`self.Dust Particles Density`)))))))