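; Configurable western town shop sign, built entirely in the construction script with no runtime logic.
; A decal projects the chosen text with adjustable offset, depth, scale and sort order.
; Each text option picks one of three parent materials plus an RGBA channel mask, so each material holds four names, tinted through a dynamic instance.
; Unless hidden, a mesh of the selected sign type is added with configurable scale and frame and main materials.
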(fn `UserConstructionScript`
  (bind _sign_scale (`self.Sign Scale`))
  (bind _text_roughness (`self.Text Roughness`))
  (bind _text_color (`self.Text Color`))
  (bind _mask (`self.Mask`))
  (bind _text_scale (`self.Text Scale`))
  (`|ExecutionSequence`
    (:`then_0`
      (bind _returnvalue (`AddComponent|NODE_AddDecalComponent-0` :`RelativeTransform` (`KismetMathLibrary.MakeTransform` (`KismetMathLibrary.MakeVector` (/ (`self.Text X Offset`) 10.0) (/ (`self.Text Projection Offset`) 10.0) (/ (`self.Text Y Offset`) 10.0)) (struct :`Yaw` 90.0 :`Roll` 90.0) (`KismetMathLibrary.MakeVector` (* 0.05 (`self.Text Projection Depth`)) _text_scale _text_scale))))
      (`DecalComponent.SetSortOrder` _returnvalue (`self.Decal Sort Order`))
      (switch `/Game/WesternDesertTown/Blueprint/BlueprintExtra/ENUM_SignText` (`self.Text`)
        (:`NewEnumerator0`
          (set `self.Mask` (struct :`R` 1.0))
          (bind _returnvalue_2 (`KismetMaterialLibrary.CreateDynamicMaterialInstance` "/Game/WesternDesertTown/Material/MI_Text01.MI_Text01" :!label _label))
          (`DecalComponent.SetDecalMaterial` _returnvalue _returnvalue_2)
          (`MaterialInstanceDynamic.SetVectorParameterValue` _returnvalue_2 "Color" _text_color)
          (`MaterialInstanceDynamic.SetVectorParameterValue` _returnvalue_2 "Mask Channel" _mask)
          (`MaterialInstanceDynamic.SetScalarParameterValue` _returnvalue_2 "Roughness" _text_roughness))
        (:`NewEnumerator1`
          (set `self.Mask` (struct :`G` 1.0))
          (goto _label))
        (:`NewEnumerator2`
          (set `self.Mask` (struct :`B` 1.0))
          (goto _label))
        (:`NewEnumerator3`
          (set `self.Mask` (struct :`A` 1.0))
          (goto _label))
        (:`NewEnumerator4`
          (set `self.Mask` (struct :`R` 1.0))
          (bind _returnvalue_3 (`KismetMaterialLibrary.CreateDynamicMaterialInstance` "/Game/WesternDesertTown/Material/MI_Text02.MI_Text02" :!label _label_2))
          (`DecalComponent.SetDecalMaterial` _returnvalue _returnvalue_3)
          (`MaterialInstanceDynamic.SetVectorParameterValue` _returnvalue_3 "Color" _text_color)
          (`MaterialInstanceDynamic.SetVectorParameterValue` _returnvalue_3 "Mask Channel" _mask)
          (`MaterialInstanceDynamic.SetScalarParameterValue` _returnvalue_3 "Roughness" _text_roughness))
        (:`NewEnumerator5`
          (set `self.Mask` (struct :`G` 1.0))
          (goto _label_2))
        (:`NewEnumerator6`
          (set `self.Mask` (struct :`B` 1.0))
          (goto _label_2))
        (:`NewEnumerator7`
          (set `self.Mask` (struct :`A` 1.0))
          (goto _label_2))
        (:`NewEnumerator8`
          (set `self.Mask` (struct :`R` 1.0))
          (bind _returnvalue_4 (`KismetMaterialLibrary.CreateDynamicMaterialInstance` "/Game/WesternDesertTown/Material/MI_Text03.MI_Text03" :!label _label_3))
          (`DecalComponent.SetDecalMaterial` _returnvalue _returnvalue_4)
          (`MaterialInstanceDynamic.SetVectorParameterValue` _returnvalue_4 "Color" _text_color)
          (`MaterialInstanceDynamic.SetVectorParameterValue` _returnvalue_4 "Mask Channel" _mask)
          (`MaterialInstanceDynamic.SetScalarParameterValue` _returnvalue_4 "Roughness" _text_roughness))
        (:`NewEnumerator9`
          (set `self.Mask` (struct :`G` 1.0))
          (goto _label_3))
        (:`NewEnumerator10`
          (set `self.Mask` (struct :`B` 1.0))
          (goto _label_3))
        (:`NewEnumerator11`
          (set `self.Mask` (struct :`A` 1.0))
          (goto _label_3))))
    (:`then_1`
      (if (not (`self.Hide Sign`))
        (switch `int` (`self.Sign Type`)
          (:`1`
            (set `self.Sign` "/Game/WesternDesertTown/Mesh/Signs/SM_Sign01.SM_Sign01"))
          (:`2`
            (set `self.Sign` "/Game/WesternDesertTown/Mesh/Signs/SM_Sign02.SM_Sign02")))
        (bind _returnvalue_5 (`AddComponent|NODE_AddStaticMeshComponent-0` :`RelativeTransform` (`KismetMathLibrary.MakeTransform` (0.0 0.0 0.0) (struct) (`KismetMathLibrary.MakeVector` _sign_scale _sign_scale _sign_scale))))
        (`StaticMeshComponent.SetStaticMesh` _returnvalue_5 (`self.Sign`))
        (`PrimitiveComponent.SetMaterial` _returnvalue_5 0 (`self.Sign Frame Material`))
        (`PrimitiveComponent.SetMaterial` _returnvalue_5 1 (`self.Sign Main Material`))))))