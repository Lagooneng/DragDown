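; BP_DirtDecal is a configurable dirt decal actor from the WesternDesertTown content.
; Its construction script adds a decal component, scaled by projection depth and decal size, with a set sort order and a dynamic instance of MI_DirtDecal.
; Exposed variables drive saturation, brightness and mask intensity, while a channel index becomes a one-hot RGBA vector selecting the mask channel.
; The event graph contains no active logic.
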(fn `UserConstructionScript`
  (bind _decal_scale (`self.Decal Scale`))
  (switch `int` (`self.Mask Channel`)
    (:`1`
      (set `self.Masks` (struct :`R` 1.0)))
    (:`2`
      (set `self.Masks` (struct :`G` 1.0)))
    (:`3`
      (set `self.Masks` (struct :`B` 1.0)))
    (:`4`
      (set `self.Masks` (struct :`A` 1.0))))
  (bind _returnvalue (`KismetMaterialLibrary.CreateDynamicMaterialInstance` "/Game/WesternDesertTown/Material/MI_DirtDecal.MI_DirtDecal"))
  (bind _returnvalue_2 (`AddComponent|NODE_AddDecalComponent-0` :`RelativeTransform` (`KismetMathLibrary.MakeTransform` (0.0 0.0 0.0) (struct :`Pitch` 270.0) (`KismetMathLibrary.MakeVector` (* 0.05 (`self.Decal Projection Depth`)) _decal_scale _decal_scale))))
  (`DecalComponent.SetSortOrder` _returnvalue_2 (`self.Decal Sort Order`))
  (`DecalComponent.SetDecalMaterial` _returnvalue_2 _returnvalue)
  (`MaterialInstanceDynamic.SetVectorParameterValue` _returnvalue "Color Adjustments" (make `LinearColor` 0.0 (`self.Decal Saturation`) (`self.Decal Brightness`)))
  (`MaterialInstanceDynamic.SetVectorParameterValue` _returnvalue "Mask Channel" (`self.Masks`))
  (`MaterialInstanceDynamic.SetScalarParameterValue` _returnvalue "Mask Intensity" (`self.Mask Intensity`)))