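; Elevator actor that toggles its cabin between two positions each time a Character enters its trigger.
; A FlipFlop alternates two MoveComponentTo nodes, stopping the opposite move before sending the cabin to a hardcoded relative location or back to StartRelativeLocation, with rotation.
; A steam sound fades in when a move starts and fades out when it completes.
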(event `self.SM_ElevatorTrigger.OnComponentBeginOverlap`
  (params (OverlappedComponent :type "PrimitiveComponent Object Reference") (OtherActor :type "Actor Object Reference") (OtherComp :type "PrimitiveComponent Object Reference") (OtherBodyIndex :type Integer) (bFromSweep :type Boolean) (SweepResult :type "HitResult Structure (by ref)"))
  (bind _elevatorcabin (`self.ElevatorCabin`))
  (bind _over_time (`self.Over Time`))
  (cast `Character` OtherActor)
  (`/Engine/EditorBlueprintResources/StandardMacros.FlipFlop`
    (:`A`
      (`|ExecutionSequence`
        (:`then_0`
          (goto _label_2 :!via `Stop`))
        (:`then_1`
          (`AudioComponent.FadeIn` (`self.Steam01_Cue`) 0.1 1.0 0.0 "Linear")
          (`KismetSystemLibrary.MoveComponentTo` _elevatorcabin (680.0 -955.0 -817.0) (`self.StartRotation`) false false _over_time :!label _label))))
    (:`B`
      (`|ExecutionSequence`
        (:`then_0`
          (goto _label :!via `Stop`))
        (:`then_1`
          (`AudioComponent.FadeIn` (`self.Steam01_Cue`) 0.1 1.0 0.0 "Linear")
          (`KismetSystemLibrary.MoveComponentTo` _elevatorcabin (`self.StartRelative Location`) (`self.EndRotation`) false false _over_time :!label _label_2)))))
  (`AudioComponent.FadeOut` (`self.Steam01_Cue`) 0.1 0.0 "Linear"))

(fn `UserConstructionScript`)