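; Wallrun_BP is a wall-run trigger actor with two collision volumes, Coll_1 and Coll_2, that mark the endpoints of a run in either direction.
; Entering either volume sends SetWRunMessage to the overlapping actor with that volume's transform as start, the opposite volume's location as target, and a left/right flag.
; Leaving either volume sends the same message with default values.
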(event `self.Coll_1.OnComponentEndOverlap`
  (params (OverlappedComponent :type "PrimitiveComponent Object Reference") (OtherActor :type "Actor Object Reference") (OtherComp :type "PrimitiveComponent Object Reference") (OtherBodyIndex :type Integer))
  ;[1 1 1] Inverse
  (message `/Game/footstepsbundle/BLUEPRINT/Wallrun_interface_BP.Set_W_Run` OtherActor false (struct) (0.0 0.0 0.0) false))

(event `self.Coll_1.OnComponentBeginOverlap`
  (params (OverlappedComponent :type "PrimitiveComponent Object Reference") (OtherActor :type "Actor Object Reference") (OtherComp :type "PrimitiveComponent Object Reference") (OtherBodyIndex :type Integer) (bFromSweep :type Boolean) (SweepResult :type "HitResult Structure (by ref)"))
  ;[1 1 1] Inverse
  (message `/Game/footstepsbundle/BLUEPRINT/Wallrun_interface_BP.Set_W_Run` OtherActor true (`SceneComponent.K2_GetComponentToWorld` (`self.Coll_1`)) (`SceneComponent.K2_GetComponentLocation` (`self.Coll_2`)) true))

(event `self.Coll_2.OnComponentBeginOverlap`
  (params (OverlappedComponent :type "PrimitiveComponent Object Reference") (OtherActor :type "Actor Object Reference") (OtherComp :type "PrimitiveComponent Object Reference") (OtherBodyIndex :type Integer) (bFromSweep :type Boolean) (SweepResult :type "HitResult Structure (by ref)"))
  ;[1 1 1] Reverse
  (message `/Game/footstepsbundle/BLUEPRINT/Wallrun_interface_BP.Set_W_Run` OtherActor true (`SceneComponent.K2_GetComponentToWorld` (`self.Coll_2`)) (`SceneComponent.K2_GetComponentLocation` (`self.Coll_1`)) false))

(event `self.Coll_2.OnComponentEndOverlap`
  (params (OverlappedComponent :type "PrimitiveComponent Object Reference") (OtherActor :type "Actor Object Reference") (OtherComp :type "PrimitiveComponent Object Reference") (OtherBodyIndex :type Integer))
  ;[1 1 1] Reverse
  (message `/Game/footstepsbundle/BLUEPRINT/Wallrun_interface_BP.Set_W_Run` OtherActor false (struct) (0.0 0.0 0.0) false))

(fn `UserConstructionScript`)